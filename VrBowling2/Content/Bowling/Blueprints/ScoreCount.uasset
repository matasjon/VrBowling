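; Bowling Blueprint that drives a text display announcing strikes.
; Every tick it checks the last entry in ScoreHistory and sets the TextRender to "Strike" when that value exceeds nine.
; Otherwise, or when the history is empty, it clears the text.
; Nodes for formatting the Score as text are present but unconnected.
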(event `self.ReceiveTick`
  (params (DeltaSeconds :type "Float (single-precision)"))
  (bind _textrender (`self.TextRender`))
  (bind _scorehistory (`self.ScoreHistory`))
  (if (> (`KismetArrayLibrary.Array_Length` _scorehistory) 0)
    (if (> (`|GetArrayItem` _scorehistory (`KismetArrayLibrary.Array_LastIndex` _scorehistory)) 9)
      (`TextRenderComponent.K2_SetText` _textrender "Strike")
      (else
        (`TextRenderComponent.K2_SetText` _textrender "" :!label _label)))
    (else
      (goto _label))))

(fn `UserConstructionScript`)