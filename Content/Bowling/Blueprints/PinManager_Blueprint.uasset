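; Bowling pin manager that spawns the rack of pins at BeginPlay and provides functions to clear pins from the lane.
; SpawnAllPins uses nested loops with row, column and centering offsets to place ten scaled-down Pin actors in a triangle at hardcoded world coordinates.
; RemoveFallenOverPins destroys Pin actors flagged FallenOver, while RemoveAllPins sets that flag on every pin and destroys it.
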(event `self.ReceiveBeginPlay`
  (`self.SpawnAllPins`))

(fn `RemoveAllPins`
  (bind _outactors (`GameplayStatics.GetAllActorsOfClass` "/Game/Bowling/Blueprints/Pin.Pin_C"))
  (for _array_element _outactors
    (set `/Game/Bowling/Blueprints/Pin.FallenOver` true _array_element)
    (`self.K2_DestroyActor` _array_element)))

(fn `RemoveFallenOverPins`
  (bind _outactors (`GameplayStatics.GetAllActorsOfClass` "/Game/Bowling/Blueprints/Pin.Pin_C"))
  (for _array_element _outactors
    (if (`/Game/Bowling/Blueprints/Pin.FallenOver` _array_element)
      (`self.K2_DestroyActor` _array_element))))

(fn `SpawnAllPins`
  (locals (StartXPos :type "Float (double-precision)") (StartYPos :type "Float (double-precision)") (RowOffset :type "Float (double-precision)") (ColOffset :type "Float (double-precision)") (MoveBy :type "Float (double-precision)"))
  (set `local.StartXPos` 1840.0)
  (set `local.StartYPos` 490.0)
  (set `local.RowOffset` 40.0)
  (set `local.ColOffset` 40.0)
  (set `local.MoveBy` -20.0)
  (for _index (range 4)
    (for _index_2 (range (+ _index 1))
      (`|SpawnActorFromClass` "/Game/Bowling/Blueprints/Pin.Pin_C" (`KismetMathLibrary.MakeTransform` (`KismetMathLibrary.MakeVector` (+ (`local.StartXPos`) (* (`local.RowOffset`) _index)) (+ (`local.StartYPos`) (* (`local.ColOffset`) _index_2) (* (`local.MoveBy`) _index)) 160.0) (struct) (0.2 0.2 0.2)) "Undefined" "OverrideRootScale" null null) ; Pin
    )))

(fn `UserConstructionScript`)