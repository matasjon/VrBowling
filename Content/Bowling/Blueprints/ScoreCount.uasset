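; Bowling score display that shows the current Score on a TextRender component.
; Every Tick it rewrites the text, showing just Score while ScoreHistory is empty.
; Otherwise it runs an empty loop over ScoreHistory and uses the element left after completion, the last entry, appended in brackets with at least two digits.
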(event `self.ReceiveTick`
  (params (DeltaSeconds :type "Float (single-precision)"))
  (bind _textrender (`self.TextRender`))
  (bind _score (`self.Score`))
  (bind _scorehistory (`self.ScoreHistory`))
  (if (> (`KismetArrayLibrary.Array_Length` _scorehistory) 0)
    (for _array_element _scorehistory
      _)
    (`TextRenderComponent.K2_SetText` _textrender (`KismetTextLibrary.Conv_StringToText` (`KismetStringLibrary.Concat_StrStr` (`KismetStringLibrary.Conv_IntToString` _score) " [" (`KismetTextLibrary.Conv_TextToString` (`KismetTextLibrary.Conv_IntToText` _array_element false true 2)) "]")))
    (else
      (`TextRenderComponent.K2_SetText` _textrender (`KismetTextLibrary.Conv_IntToText` _score)))))

(fn `UserConstructionScript`)