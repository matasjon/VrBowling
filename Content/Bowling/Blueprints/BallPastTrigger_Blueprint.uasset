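; Trigger actor in the bowling game that ends each shot when a ball overlaps it.
; After a delay for pins to fall, it records the ScoreCount score and spawns a scoreboard text item positioned by turn and shot.
; A score of ten or a second shot respawns all pins through PinManager and advances the turn; otherwise fallen pins are removed.
; It then resets the score; the ball's destroy call is noted as not working.
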(event `self.ReceiveActorBeginOverlap`
  (params (OtherActor :type "Actor Object Reference"))
  (cast `/Game/Bowling/Blueprints/ball` OtherActor)
  (`KismetSystemLibrary.Delay` 5.0) ; Should be long enough to ensure\nthere's always time for pins to fall down
  (`self.K2_DestroyActor` OtherActor) ; Somewhy does not work
  (bind _returnvalue (`GameplayStatics.GetActorOfClass` "/Game/Bowling/Blueprints/ScoreCount.ScoreCount_C"))
  (bind _score (`/Game/Bowling/Blueprints/ScoreCount.Score` _returnvalue))
  (`KismetArrayLibrary.Array_Add` (`/Game/Bowling/Blueprints/ScoreCount.ScoreHistory` _returnvalue) _score)
  (bind _turncount (`/Game/Bowling/Blueprints/ScoreCount.TurnCount` _returnvalue))
  (bind _secondshot (`/Game/Bowling/Blueprints/ScoreCount.SecondShot` _returnvalue))
  (bind _returnvalue_2 (`|SpawnActorFromClass` "/Game/Bowling/Blueprints/ScoreboardItem_Blueprint.ScoreboardItem_Blueprint_C" (`KismetMathLibrary.MakeTransform` (`KismetMathLibrary.MakeVector` 210.0 (+ 320.0 (* _turncount 20.0)) (+ 280.0 (* 20.0 (`KismetMathLibrary.Conv_BoolToInt` _secondshot)))) (struct :`Yaw` 180.0)) "Undefined" "OverrideRootScale" null null))
  (`TextRenderComponent.K2_SetText` (`/Game/Bowling/Blueprints/ScoreboardItem_Blueprint.TextRender` _returnvalue_2) (`KismetTextLibrary.Conv_IntToText` _score))
  (bind _returnvalue_3 (`GameplayStatics.GetActorOfClass` "/Game/Bowling/Blueprints/PinManager_Blueprint.PinManager_Blueprint_C"))
  (if (>= _score 10)
    (`/Game/Bowling/Blueprints/PinManager_Blueprint.RemoveAllPins` _returnvalue_3 :!label _label)
    (`/Game/Bowling/Blueprints/PinManager_Blueprint.SpawnAllPins` _returnvalue_3)
    (set `/Game/Bowling/Blueprints/ScoreCount.TurnCount` (+ _turncount 1) _returnvalue)
    (set `/Game/Bowling/Blueprints/ScoreCount.SecondShot` false _returnvalue)
    (elif _secondshot
      (goto _label)
      (else
        (`/Game/Bowling/Blueprints/PinManager_Blueprint.RemoveFallenOverPins` _returnvalue_3)
        (set `/Game/Bowling/Blueprints/ScoreCount.SecondShot` true _returnvalue))))
  (set `/Game/Bowling/Blueprints/ScoreCount.Score` 0 _returnvalue))

(fn `UserConstructionScript`)